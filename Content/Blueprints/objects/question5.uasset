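; Question actor that displays a question with yes and no answer texts in the world when something enters its trigger box.
; BeginPlay hides the three text components.
; Any overlap with the Box makes them visible and fills them from the Question, Question1yes and Question1no variables.
; There is no end-overlap or answer-handling logic, so the texts stay visible once shown.
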(event OnComponentBeginOverlap(Box)
  (params (OverlappedComponent :type Primitive%20Component%20Object%20Reference) (OtherActor :type Actor%20Object%20Reference) (OtherComp :type Primitive%20Component%20Object%20Reference) (OtherBodyIndex :type Integer) (bFromSweep :type Boolean) (SweepResult :type Hit%20Result%20Structure%20%28by%20ref%29))
  ;[1 1 1] set vis
  (Utilities|FlowControl|Sequence
    (:then_0
      (Rendering|SetVisibility (Variables|Default|Gettextrender) true false)
      (Rendering|Components|TextRender|SetText (Variables|Default|Gettextrender) (Utilities|Text|ToText(String) (Variables|Default|Getquestion))))
    (:then_1
      (Rendering|SetVisibility (Variables|Default|Gettext_yes) true false)
      (Rendering|Components|TextRender|SetText (Variables|Default|Gettext_yes) (Utilities|Text|ToText(String) (Variables|Default|Getquestion1yes))))
    (:then_2
      (Rendering|SetVisibility (Variables|Default|Gettext_no) true false)
      (Rendering|Components|TextRender|SetText (Variables|Default|Gettext_no) (Utilities|Text|ToText(String) (Variables|Default|Getquestion1no))))))

(event Collision|EventActorBeginOverlap
  (params (OtherActor :type Actor%20Object%20Reference)))

(event EventTick
  (params (DeltaSeconds :type Float%20%28single-precision%29)))

(event EventBeginPlay
  ;[1 1 1] set invis
  (Utilities|FlowControl|Sequence
    (:then_0
      (Rendering|SetVisibility (Variables|Default|Gettextrender) false false))
    (:then_1
      (Rendering|SetVisibility (Variables|Default|Gettext_yes) false false))
    (:then_2
      (Rendering|SetVisibility (Variables|Default|Gettext_no) false false))))

(fn ConstructionScript)