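; Spot actor for a waiting challenge where the player wins once a 60-second timer expires, showing Winner widgets.
; The Timer trigger starts named timers for that win and for five "rush" popups at 10-second intervals.
; Option1 and Option2 triggers restart those timers and show wrong-answer feedback, with Option2 also calling Teleport to the origin on the player controller.
; A separate Box trigger lowers the wall group once via a timeline.
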(event OnComponentBeginOverlap(timer)
  (params (OverlappedComponent :type Primitive%20Component%20Object%20Reference) (OtherActor :type Actor%20Object%20Reference) (OtherComp :type Primitive%20Component%20Object%20Reference) (OtherBodyIndex :type Integer) (bFromSweep :type Boolean) (SweepResult :type Hit%20Result%20Structure%20%28by%20ref%29))
  ;[1 1 1] timer at end with rushes
  (Utilities|FlowControl|Sequence
    (:then_0
      (Utilities|Time|ClearTimerbyFunctionName 0 "quitgame")
      (Utilities|Time|SetTimerbyFunctionName 0 "quitgame" 6e+01))
    (:then_1
      (Utilities|Time|ClearTimerbyFunctionName 0 "rush1")
      (Utilities|Time|SetTimerbyFunctionName 0 "rush1" 1e+01))
    (:then_2
      (Utilities|Time|ClearTimerbyFunctionName 0 "rush2")
      (Utilities|Time|SetTimerbyFunctionName 0 "rush2" 2e+01))
    (:then_3
      (Utilities|Time|ClearTimerbyFunctionName 0 "rush3")
      (Utilities|Time|SetTimerbyFunctionName 0 "rush3" 3e+01))
    (:then_4
      (Utilities|Time|ClearTimerbyFunctionName 0 "rush4")
      (Utilities|Time|SetTimerbyFunctionName 0 "rush4" 4e+01))
    (:then_5
      (Utilities|Time|ClearTimerbyFunctionName 0 "rule5")
      (Utilities|Time|SetTimerbyFunctionName 0 "rush5" 5e+01))))

(event OnComponentBeginOverlap(option1)
  (params (OverlappedComponent :type Primitive%20Component%20Object%20Reference) (OtherActor :type Actor%20Object%20Reference) (OtherComp :type Primitive%20Component%20Object%20Reference) (OtherBodyIndex :type Integer) (bFromSweep :type Boolean) (SweepResult :type Hit%20Result%20Structure%20%28by%20ref%29))
  ;[1 1 1] blah widget and reset timer
  (Utilities|FlowControl|Sequence
    (:then_0
      (Utilities|Time|ClearTimerbyFunctionName 0 "quitgame")
      (Utilities|Time|SetTimerbyFunctionName 0 "quitgame" 6e+01))
    (:then_1
      (Utilities|Time|ClearTimerbyFunctionName 0 "rush1")
      (Utilities|Time|SetTimerbyFunctionName 0 "rush1" 1e+01))
    (:then_2
      (Utilities|Time|ClearTimerbyFunctionName 0 "rush2")
      (Utilities|Time|SetTimerbyFunctionName 0 "rush2" 2e+01))
    (:then_3
      (Utilities|Time|ClearTimerbyFunctionName 0 "rush3")
      (Utilities|Time|SetTimerbyFunctionName 0 "rush3" 3e+01))
    (:then_4
      (Utilities|Time|ClearTimerbyFunctionName 0 "rush4")
      (Utilities|Time|SetTimerbyFunctionName 0 "rush4" 4e+01))
    (:then_5
      (Utilities|Time|ClearTimerbyFunctionName 0 "rule5")
      (Utilities|Time|SetTimerbyFunctionName 0 "rush5" 5e+01))
    (:then_6
      (Utilities|FlowControl|Delay 2.0)
      (Utilities|FlowControl|Sequence
        (:then_0
          (bind _returnvalue (UserInterface|CreateWidget "/Game/Blueprints/widgets/blah.blah_C"))
          (bind _output_get (Variables|Default|Setblah _returnvalue))
          (UserInterface|Viewport|AddtoViewport _output_get 0)
          (Utilities|FlowControl|Delay 5.0)
          (Viewport|RemoveAllWidgets))
        (:then_1
          (Audio|PlaySound2D "/Game/Blueprints/audio/incorrect_sound_effect.incorrect_sound_effect" 1.0 1.0 0.0 0 0))))))

(event OnComponentBeginOverlap(Box)
  (params (OverlappedComponent :type Primitive%20Component%20Object%20Reference) (OtherActor :type Actor%20Object%20Reference) (OtherComp :type Primitive%20Component%20Object%20Reference) (OtherBodyIndex :type Integer) (bFromSweep :type Boolean) (SweepResult :type Hit%20Result%20Structure%20%28by%20ref%29))
  ;[1 1 1] removes walls
  ;;[1 1 1] sliding door sound
  (Utilities|FlowControl|DoOnce false
    (:Completed
      (Audio|PlaySound2D "/Game/Blueprints/audio/slidingdoor.slidingdoor" 1.0 1.0 0.0 0 0)
      (bind _newtrack_0 (Timeline|wallsdown Play)
        (:Update
          (Transformation|SetRelativeLocation (Variables|Default|Getboxgroup) (Math|Vector|Lerp(Vector) "0, 0, 0" "0, 0,-2100.000000" _newtrack_0) false false))))))

(event OnComponentBeginOverlap(option2)
  (params (OverlappedComponent :type Primitive%20Component%20Object%20Reference) (OtherActor :type Actor%20Object%20Reference) (OtherComp :type Primitive%20Component%20Object%20Reference) (OtherBodyIndex :type Integer) (bFromSweep :type Boolean) (SweepResult :type Hit%20Result%20Structure%20%28by%20ref%29))
  ;[1 1 1] blah widget and reset timer
  (Utilities|FlowControl|Sequence
    (:then_0
      (Utilities|Time|ClearTimerbyFunctionName 0 "quitgame")
      (Utilities|Time|SetTimerbyFunctionName 0 "quitgame" 6e+01))
    (:then_1
      (Utilities|Time|ClearTimerbyFunctionName 0 "rush1")
      (Utilities|Time|SetTimerbyFunctionName 0 "rush1" 1e+01))
    (:then_2
      (Utilities|Time|ClearTimerbyFunctionName 0 "rush2")
      (Utilities|Time|SetTimerbyFunctionName 0 "rush2" 2e+01))
    (:then_3
      (Utilities|Time|ClearTimerbyFunctionName 0 "rush3")
      (Utilities|Time|SetTimerbyFunctionName 0 "rush3" 3e+01))
    (:then_4
      (Utilities|Time|ClearTimerbyFunctionName 0 "rush4")
      (Utilities|Time|SetTimerbyFunctionName 0 "rush4" 4e+01))
    (:then_5
      (Utilities|Time|ClearTimerbyFunctionName 0 "rule5")
      (Utilities|Time|SetTimerbyFunctionName 0 "rush5" 5e+01))
    (:then_6
      (Utilities|FlowControl|Delay 2.0)
      (Utilities|FlowControl|Sequence
        (:then_0
          (bind _returnvalue (UserInterface|CreateWidget "/Game/Blueprints/widgets/blah1.blah1_C"))
          (bind _output_get (Variables|Default|Setblah1 _returnvalue))
          (UserInterface|Viewport|AddtoViewport _output_get 0)
          (Utilities|FlowControl|Delay 5.0)
          (Utilities|FlowControl|Sequence
            (:then_0
              (Viewport|RemoveAllWidgets))
            (:then_1
              (Transformation|Teleport (Game|GetPlayerController 0) "0, 0, 0" "0, 0, 0"))))
        (:then_1
          (Audio|PlaySound2D "/Game/Blueprints/audio/incorrect_sound_effect.incorrect_sound_effect" 1.0 1.0 0.0 0 0))))))

(event Custom|quitgame
  ;[1 1 1] timer at end with rushes
  (bind _returnvalue (UserInterface|CreateWidget "/Game/Blueprints/widgets/winner.winner_C"))
  (bind _output_get (Variables|Default|Setwinner _returnvalue))
  (UserInterface|Viewport|AddtoViewport _output_get 0)
  (Utilities|FlowControl|Delay 2.0)
  (Audio|PlaySound2D "/Game/Blueprints/audio/tada.tada" 1.0 1.0 0.0 0 0)
  (bind _returnvalue_2 (UserInterface|CreateWidget "/Game/Blueprints/widgets/winner1.winner1_C"))
  (bind _output_get_2 (Variables|Default|Setwinner1 _returnvalue_2))
  (UserInterface|Viewport|AddtoViewport _output_get_2 0)
  (Variables|/Script/Engine.PlayerController|SetbShowMouseCursor (Game|GetPlayerController 0) true))

(event Custom|rush1
  ;[1 1 1] timer at end with rushes
  (bind _returnvalue (UserInterface|CreateWidget "/Game/Blueprints/widgets/rush1.rush1_C"))
  (bind _output_get (Variables|Default|Setrush11 _returnvalue))
  (UserInterface|Viewport|AddtoViewport _output_get 0)
  (Utilities|FlowControl|Delay 3.0)
  (Viewport|RemoveAllWidgets))

(event Custom|rush2
  ;[1 1 1] timer at end with rushes
  (bind _returnvalue (UserInterface|CreateWidget "/Game/Blueprints/widgets/rush2.rush2_C"))
  (bind _output_get (Variables|Default|Setrush22 _returnvalue))
  (UserInterface|Viewport|AddtoViewport _output_get 0)
  (Utilities|FlowControl|Delay 3.0)
  (Viewport|RemoveAllWidgets))

(event Custom|rush3
  ;[1 1 1] timer at end with rushes
  (bind _returnvalue (UserInterface|CreateWidget "/Game/Blueprints/widgets/rush3.rush3_C"))
  (bind _output_get (Variables|Default|Setrush33 _returnvalue))
  (UserInterface|Viewport|AddtoViewport _output_get 0)
  (Utilities|FlowControl|Delay 3.0)
  (Viewport|RemoveAllWidgets))

(event Custom|rush4
  ;[1 1 1] timer at end with rushes
  (bind _returnvalue (UserInterface|CreateWidget "/Game/Blueprints/widgets/rush4.rush4_C"))
  (bind _output_get (Variables|Default|Setrush44 _returnvalue))
  (UserInterface|Viewport|AddtoViewport _output_get 0)
  (Utilities|FlowControl|Delay 3.0)
  (Viewport|RemoveAllWidgets))

(event Custom|rush5
  ;[1 1 1] timer at end with rushes
  (bind _returnvalue (UserInterface|CreateWidget "/Game/Blueprints/widgets/rush5.rush5_C"))
  (bind _output_get (Variables|Default|Setrush55 _returnvalue))
  (UserInterface|Viewport|AddtoViewport _output_get 0)
  (Utilities|FlowControl|Delay 3.0)
  (Viewport|RemoveAllWidgets))

(event Collision|EventActorBeginOverlap
  (params (OtherActor :type Actor%20Object%20Reference)))

(event EventTick
  (params (DeltaSeconds :type Float%20%28single-precision%29)))

(event EventBeginPlay
  ;[1 1 1] idk tbh
  (Rendering|Components|TextRender|SetText (Variables|Default|GetTextRender) (Utilities|Text|ToText(String) (Variables|Default|Getstand))))

(fn ConstructionScript)