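; Elevator platform that, once triggered by an overlap, plays an incorrect-answer sound and an elevator sound while dropping.
; Two seconds after the box overlap, a DoOnce starts a timeline that lerps the cube downward.
; The timeline's Update also runs a delay that snaps the cube back to its origin.
; In parallel it shows the No4 widget, then removes all widgets five seconds later.
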(event OnComponentBeginOverlap(Box)
  (params (OverlappedComponent :type Primitive%20Component%20Object%20Reference) (OtherActor :type Actor%20Object%20Reference) (OtherComp :type Primitive%20Component%20Object%20Reference) (OtherBodyIndex :type Integer) (bFromSweep :type Boolean) (SweepResult :type Hit%20Result%20Structure%20%28by%20ref%29))
  ;[1 1 1] moves platform, sets it back, and creates hud
  (Utilities|FlowControl|Delay 2.0)
  ;[1 1 1] audio rr rr
  (Utilities|FlowControl|DoOnce false
    (:Completed
      (Audio|PlaySound2D "/Game/Blueprints/audio/incorrect_sound_effect.incorrect_sound_effect" 1.0 1.0 0.0 0 0)
      (Audio|PlaySound2D "/Game/Blueprints/audio/elevatorsound.elevatorsound" 1.0 1.0 0.0 0 0)
      (Utilities|FlowControl|Sequence
        (:then_0
          (bind _newtrack_0 (Timeline|Timeline_0 Play)
            (:Update
              (Transformation|SetRelativeLocation (Variables|Default|GetCube) (Math|Vector|Lerp(Vector) "0, 0, 0" "0, 0,-550.000000" _newtrack_0) false false)
              (Utilities|FlowControl|Delay 2.0)
              (Transformation|SetRelativeLocation (Variables|Default|GetCube) (Math|Vector|Lerp(Vector) "0, 0, 0" "0, 0, 0" 0.0) false false))))
        (:then_1
          (bind _returnvalue (UserInterface|CreateWidget "/Game/Blueprints/widgets/no4.no4_C"))
          (bind _output_get (Variables|Default|Setno4 _returnvalue))
          (UserInterface|Viewport|AddtoViewport _output_get 0)
          (Utilities|FlowControl|Delay 5.0)
          (Viewport|RemoveAllWidgets))))))

(event EventBeginPlay)

(event Collision|EventActorBeginOverlap
  (params (OtherActor :type Actor%20Object%20Reference)))

(event EventTick
  (params (DeltaSeconds :type Float%20%28single-precision%29)))

(fn ConstructionScript)